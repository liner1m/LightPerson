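; BPC_Lighter is a Blueprint component that, despite its name, tracks a health value between zero and a maximum.
; It fills Health on BeginPlay and offers functions to damage, add, fully recover and query it, including as a fraction.
; Changes broadcast the EDChange dispatcher, and reaching zero calls OnDead through a DoOnce that is never reset, even by Recovery.
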(event `self.ReceiveBeginPlay`
  (`self.recovery`)
  (`self.ED_Change`))

(fn `Add Health`
  (params (add :type "Float (double-precision)"))
  (set `self.health` (`KismetMathLibrary.FMin` (+ add (`self.health`)) (`self.maxHealth`)))
  (`self.ED_Change`))

(fn `damage`
  (params (damage :type "Float (double-precision)"))
  (bind _output_get (set `self.health` (`KismetMathLibrary.FMax` (- (`self.health`) damage))))
  (`self.ED_Change`)
  (if (== _output_get 0.0)
    (`/Engine/EditorBlueprintResources/StandardMacros.DoOnce` false
      (:`Completed`
        (`self.OnDead`)
        (`self.ED_Change`)))))

(fn `get health`
  (returns (health :type "Float (double-precision)"))
  (return (`self.health`)))

(fn `getPercentHealth`
  (returns (ReturnValue :type "Float (double-precision)"))
  (return (/ (`self.health`) (`self.maxHealth`))))

(fn `is dead`
  (returns (yes :type Boolean))
  (return (== (`self.health`) 0.0)))

(fn `recovery`
  (set `self.health` (`self.maxHealth`))
  (`self.ED_Change`))